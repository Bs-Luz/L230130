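; BP_P38 is a player-controlled P-38 plane pawn that constantly flies forward and spins its two propellers every tick.
; BeginPlay adds the IMC_Input Enhanced Input context, whose pitch-and-roll action feeds controller rotation input.
; The fire action spawns an actor at the Arrow component's transform, though the live spawn shows no class.
; Legacy axis events are empty, disconnected older logic remains, and the RotatePropeller helper is not called.
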(event Input|EnhancedActionEvents|EnhancedInputActionIA_Fire
  (params (ActionValue :type Boolean) (ElapsedSeconds :type Float%20%28double-precision%29) (TriggeredSeconds :type Float%20%28double-precision%29) (InputAction :type Input%20Action%20Object%20Reference :default "/Game/Blueprints/Input/IA_Fire.IA_Fire"))
  ;[0 0 0] 향상된 입력 시스템
  (:Triggered
    (Game|SpawnActorfromClass "/Game/Blueprints/BP_Rocket.BP_Rocket_C" (Transformation|GetWorldTransform (Variables|Default|GetArrow)) "AdjustIfPossibleButDontSpawnIfColliding" 0 0)))

(event Input|EnhancedActionEvents|EnhancedInputActionIA_Pitch
  (params (ActionValue :type Float%20%28double-precision%29) (ElapsedSeconds :type Float%20%28double-precision%29) (TriggeredSeconds :type Float%20%28double-precision%29) (InputAction :type Input%20Action%20Object%20Reference :default "/Game/Blueprints/Input/IA_Pitch.IA_Pitch"))
  ;[0 0 0] 향상된 입력 시스템
)

(event Input|EnhancedActionEvents|EnhancedInputActionIA_Roll
  (params (ActionValue :type Float%20%28double-precision%29) (ElapsedSeconds :type Float%20%28double-precision%29) (TriggeredSeconds :type Float%20%28double-precision%29) (InputAction :type Input%20Action%20Object%20Reference :default "/Game/Blueprints/Input/IA_Roll.IA_Roll"))
  ;[0 0 0] 향상된 입력 시스템
)

(event Input|EnhancedActionEvents|EnhancedInputActionIA_PitchAndRoll
  (params (ActionValue :type Vector%202D%20Structure) (ElapsedSeconds :type Float%20%28double-precision%29) (TriggeredSeconds :type Float%20%28double-precision%29) (InputAction :type Input%20Action%20Object%20Reference :default "/Game/Blueprints/Input/IA_PitchAndRoll.IA_PitchAndRoll"))
  ;[0 0 0] 향상된입력을 통해 Pitch와Roll을 함께 입력 받을 수 있다
  (:Triggered
    (Pawn|Input|AddControllerRollInput (.x ActionValue))
    (Pawn|Input|AddControllerPitchInput (.y ActionValue))))

(event EventBeginPlay
  ;[0 0 0] 향상된 입력 시스템
  (Utilities|IsValid (Game|GetPlayerController 0)
    (:Is%20Valid
      (Input|AddMappingContext (PlayerController|LocalPlayerSubsystems|GetEnhancedInputLocalPlayerSubsystem (Game|GetPlayerController 0)) "/Game/Blueprints/Input/IMC_Input.IMC_Input" 0 "(bIgnoreAllPressedKeysUntilRelease=True,bForceImmediately=False)"))))

(event EventTick
  (params (DeltaSeconds :type Float%20%28single-precision%29))
  (Pawn|Input|AddMovementInput (Transformation|GetActorForwardVector) 1.0 false)
  (Transformation|AddLocalRotation (Variables|Default|GetRightPropeller) (* (Variables|Default|GetPropllerRotateSpeed) (Utilities|Time|GetWorldDeltaSeconds)) false false)
  (Transformation|AddLocalRotation (Variables|Default|GetLeftPropeller) (* (Variables|Default|GetPropllerRotateSpeed) (Utilities|Time|GetWorldDeltaSeconds)) false false))

(event Input|ActionEvents|InputActionFire
  (params (Key :type Key%20Structure :default "None"))
  ;[0 0 0] 5.0이전의 입력 매핑 방식
)

(event Input|AxisEvents|InputAxisPitch
  (params (AxisValue :type Float%20%28single-precision%29))
  ;[0 0 0] 5.0이전의 입력 매핑 방식
)

(event Input|AxisEvents|InputAxisRoll
  (params (AxisValue :type Float%20%28single-precision%29))
  ;[0 0 0] 5.0이전의 입력 매핑 방식
)

(fn ConstructionScript)

(fn RotatePropeller
  (params (self2 :type Scene%20Component%20Object%20Reference))
  (Transformation|AddLocalRotation self2 (Math|Rotator|MakeRotator (* (Utilities|Time|GetWorldDeltaSeconds) (Variables|Default|GetPropellerSpeed)) 0.0 0.0) false false))